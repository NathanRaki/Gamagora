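; SmartBoy_BP builds a 3D maze from one of four random PNGs and tracks the player's path through it.
; BeginPlay imports the image, draws it through a dynamic material to a render target, and reads back each pixel.
; Black pixels become wall meshes over floor tiles, and the first and last open pixels set SpawnPoint and EndPoint.
; Tick maps the player's location to a grid index and paints that floor tile blue, except the end tile.
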(event `self.ReceiveBeginPlay`
  (bind _xpos (`self.xPos`))
  (bind _ypos (`self.yPos`))
  (bind _xpos_2 (`self.xPos`))
  (bind _ypos_2 (`self.yPos`))
  (bind _returnvalue (/ (`self.Distance`) -1.0))
  ;[1 1 1] Render the Texture to Target
  (bind _returnvalue_2 (`KismetMaterialLibrary.CreateDynamicMaterialInstance` "/Game/DynamicMaze_Mat.DynamicMaze_Mat"))
  (bind _output_get (set `self.DynamicMaze_Mat` _returnvalue_2))
  (bind _returnvalue_3 (`KismetRenderingLibrary.ImportFileAsTexture2D` (`KismetStringLibrary.Concat_StrStr` (`BlueprintPathsLibrary.GetPath` (`BlueprintPathsLibrary.GetProjectFilePath`)) "/maze" (`KismetStringLibrary.Conv_IntToString` (`KismetMathLibrary.RandomIntegerInRange` 1 4)) ".png")))
  (`MaterialInstanceDynamic.SetTextureParameterValue` _output_get "Texture" _returnvalue_3)
  (`KismetRenderingLibrary.DrawMaterialToRenderTarget` "/Game/16x16RenderTarget2D.16x16RenderTarget2D" _output_get)
  (bind _outactors (`GameplayStatics.GetAllActorsWithTag` "Player"))
  (set `self.Player` (`KismetArrayLibrary.Array_Random` _outactors))
  (`|ExecutionSequence`
    (:`then_0`
      ;[1 1 1] Get every pixel value
      (for _index (range (`self.Size`))
        (for _index_2 (range (`self.Size`))
          (bind _returnvalue_4 (`KismetRenderingLibrary.ReadRenderTargetPixel` "/Game/16x16RenderTarget2D.16x16RenderTarget2D" _index_2 _index))
          ;[1 1 1] Add value to pixels array
          (`KismetArrayLibrary.Array_Add` (`self.TColors`) _returnvalue_4))))
    (:`then_1`
      (for (_array_element _array_index) (`self.TColors`)
        (bind (_b _g _r) (break `Color` _array_element))
        (if (!= (`KismetMathLibrary.Conv_ByteToInt` (+ _b _g _r)) 0)
          (set `self.LastCase` _array_index)))
      (for (_array_element_2 _array_index_2) (`self.TColors`)
        (set `self.xPos` (* (mod _array_index_2 (`self.Size`)) (`self.Distance`)))
        (set `self.yPos` (* (/ _array_index_2 (`self.Size`)) (`self.Distance`)))
        (bind (_b_2 _g_2 _r_2) (break `Color` _array_element_2))
        (bind _returnvalue_5 (`KismetMathLibrary.Conv_ByteToInt` (+ _b_2 _g_2 _r_2)))
        (`KismetArrayLibrary.Array_Add` (`self.TPixels`) _returnvalue_5)
        (if (== _returnvalue_5 0)
          (`AddComponent|NODE_AddStaticMeshComponent-0` :`RelativeTransform` (`KismetMathLibrary.MakeTransform` (`KismetMathLibrary.MakeVector` (`self.xPos`) (`self.yPos`)) (struct) (`KismetMathLibrary.Conv_DoubleToVector` (/ (`self.Distance`) 100.0))))
          (bind _returnvalue_6 (`AddComponent|NODE_AddStaticMeshComponent-1` :`RelativeTransform` (`KismetMathLibrary.MakeTransform` (`KismetMathLibrary.MakeVector` (`self.xPos`) (`self.yPos`) (/ (`self.Distance`) -1.0)) (struct) (`KismetMathLibrary.Conv_DoubleToVector` (/ (`self.Distance`) 100.0))) :!label _label))
          (`KismetArrayLibrary.Array_Add` (`self.Meshes`) _returnvalue_6)
          (elif (== (`self.SpawnPoint`) (0.0 0.0 0.0))
            (bind _returnvalue_7 (`AddComponent|NODE_AddStaticMeshComponent-2` :`RelativeTransform` (`KismetMathLibrary.MakeTransform` (`KismetMathLibrary.MakeVector` _xpos_2 _ypos_2 (/ (`self.Distance`) -1.0)) (struct) (`KismetMathLibrary.Conv_DoubleToVector` (/ (`self.Distance`) 100.0)))))
            (set `self.SpawnPoint` (`KismetMathLibrary.MakeVector` _xpos_2 _ypos_2 (/ (`self.Distance`) 2.0)))
            (`KismetArrayLibrary.Array_Add` (`self.Meshes`) _returnvalue_7)
            (elif (== _array_index_2 (`self.LastCase`))
              (bind _returnvalue_8 (`AddComponent|NODE_AddStaticMeshComponent-4` :`RelativeTransform` (`KismetMathLibrary.MakeTransform` (`KismetMathLibrary.MakeVector` _xpos _ypos _returnvalue) (struct) (`KismetMathLibrary.Conv_DoubleToVector` (/ (`self.Distance`) 100.0)))))
              (set `self.EndPoint` (`KismetMathLibrary.MakeVector` _xpos _ypos _returnvalue))
              (`KismetArrayLibrary.Array_Add` (`self.Meshes`) _returnvalue_8)
              (else
                (goto _label)))))))))

(event `self.ReceiveTick`
  (params (DeltaSeconds :type "Float (single-precision)"))
  (bind (_returnvalue_x _returnvalue_y) (`KismetMathLibrary.BreakVector` (/ (+ (`self.K2_GetActorLocation` (`self.Player`)) (/ (`self.Distance`) 2.0)) (`self.Distance`))))
  (set `self.CurrentX` (`KismetMathLibrary.FTrunc` _returnvalue_x))
  (set `self.CurrentY` (`KismetMathLibrary.FTrunc` _returnvalue_y))
  (for (_array_element _array_index) (`self.Meshes`)
    (if (== _array_index (+ (* (`self.Size`) (`self.CurrentY`)) (`self.CurrentX`)))
      (if (!= _array_index (`self.LastCase`))
        (`PrimitiveComponent.SetMaterial` _array_element 0 "/Game/Blue_Mat.Blue_Mat")
        (break)
        (else
          (break))))))

(fn `UserConstructionScript`)