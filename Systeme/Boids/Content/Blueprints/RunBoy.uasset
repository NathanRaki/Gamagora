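; RunBoy is a player-controlled pawn with basic movement, mouse turning and a health pool.
; Forward and Right axis inputs move it relative to the control rotation, while mouse X drives controller yaw.
; Health starts at MaxHealth and drops by a fixed amount whenever the pawn begins overlapping a BadBoy actor, with no death handling or lower limit.
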(event `self.ReceiveBeginPlay`
  (set `self.HealthPoints` (`self.MaxHealth`)))

(event `InputAxis|Forward`
  (params (AxisValue :type "Float (single-precision)"))
  ;[1 1 1] Movements
  (`self.AddMovementInput` (`KismetMathLibrary.GetForwardVector` (`self.GetControlRotation`)) AxisValue))

(event `InputAxisKey|MouseX`
  (params (AxisValue :type "Float (single-precision)"))
  (`self.AddControllerYawInput` AxisValue))

(event `self.ReceiveActorBeginOverlap`
  (params (OtherActor :type "Actor Object Reference"))
  (cast `/Game/Blueprints/BadBoy` OtherActor)
  (set `self.HealthPoints` (- (`self.HealthPoints`) 10)))

(event `InputAxis|Right`
  (params (AxisValue :type "Float (single-precision)"))
  ;[1 1 1] Movements
  (`self.AddMovementInput` (`KismetMathLibrary.GetRightVector` (`self.GetControlRotation`)) AxisValue))

(fn `UserConstructionScript`)