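; BadBoy is an enemy character that moves as a boids-style flock relative to RunBoy, with a Die event that spawns steam and destroys it.
; Each tick it copies tuning from RunBoy_BP and combines cohesion, alignment, separation and target vectors from nearby BadBoys and RunBoy.
; RunBoy's state makes it flee, chase faster or follow a random direction chosen at BeginPlay.
; After RunBoy's Lifespan, its animation action changes and steering stops.
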(event `Die`
  (`GameplayStatics.SpawnEmitterAtLocation` "/Game/Particles/P_Steam_Lit.P_Steam_Lit" (`self.K2_GetActorLocation`))
  (`self.K2_DestroyActor`))

(event `self.ReceiveBeginPlay`
  (set `self.DirectionChanger` (`KismetMathLibrary.MakeVector` (`KismetMathLibrary.RandomFloatInRange` -1.0 1.0) (`KismetMathLibrary.RandomFloatInRange` -1.0 1.0)))
  (bind _returnvalue (`GameplayStatics.GetActorOfClass` "/Game/Blueprints/RunBoy_BP.RunBoy_BP_C"))
  (bind _asenemy_animation (cast `/Game/Blueprints/Enemy_Animation` (`SkeletalMeshComponent.GetAnimInstance` (`self.Mesh`))))
  (set `/Game/Blueprints/Enemy_Animation.Actions` "NewEnumerator1" _asenemy_animation)
  (`KismetSystemLibrary.Delay` (`/Game/Blueprints/RunBoy_BP.Lifespan` _returnvalue))
  (set `/Game/Blueprints/Enemy_Animation.Actions` "NewEnumerator2" _asenemy_animation))

(event `self.ReceiveTick`
  (params (DeltaSeconds :type "Float (single-precision)"))
  (bind _asenemy_animation (cast `/Game/Blueprints/Enemy_Animation` (`SkeletalMeshComponent.GetAnimInstance` (`self.Mesh`))))
  (if (`|EnumInequality` (`/Game/Blueprints/Enemy_Animation.Actions` _asenemy_animation) "NewEnumerator2")
    (`self.ImportVariables`)
    (bind _outactors (`GameplayStatics.GetAllActorsOfClass` "BadBoy_C"))
    (bind _output_get (set `self.OtherBadBoys` _outactors))
    (`KismetArrayLibrary.Array_RemoveItem` _output_get self)
    (bind _returnvalue (`GameplayStatics.GetActorOfClass` "/Game/Blueprints/RunBoy.RunBoy_C"))
    (bind _state (`/Game/Blueprints/RunBoy.State` _returnvalue))
    (`/Engine/EditorBlueprintResources/StandardMacros.IsValid` _state
      (:`Is Valid`
        (bind _state_2 (`/Game/Blueprints/PowerUp.State` _state))
        (if (`|EnumEquality` _state_2 "NewEnumerator1")
          (`self.Loop` -1.0)
          (elif (`|EnumEquality` _state_2 "NewEnumerator3")
            (`self.Loop` 1.0 (`self.DirectionChanger`))
            (elif (`|EnumEquality` _state_2 "NewEnumerator2")
              (`self.Loop` 1.0 (1.0 1.0 1.0) 700.0)))))
      (:`Is Not Valid`
        (`self.Loop` 1.0)))))

(fn `ImportVariables`
  (bind _returnvalue (`GameplayStatics.GetActorOfClass` "/Game/Blueprints/RunBoy_BP.RunBoy_BP_C"))
  (set `self.CloserFactor` (`/Game/Blueprints/RunBoy_BP.CloseFactor` _returnvalue))
  (set `self.WithFactor` (`/Game/Blueprints/RunBoy_BP.WithFactor` _returnvalue))
  (set `self.AwayFactor` (`/Game/Blueprints/RunBoy_BP.AwayFactor` _returnvalue))
  (set `self.TargetFactor` (`/Game/Blueprints/RunBoy_BP.TargetFactor` _returnvalue))
  (set `self.MinDistance` (`/Game/Blueprints/RunBoy_BP.MinDistance` _returnvalue))
  (set `self.CloseDistance` (`/Game/Blueprints/RunBoy_BP.CloseDistance` _returnvalue)))

(fn `Loop`
  (params (DirectionFactor :type "Float (double-precision)" :default 1.0) (DirectionChanger :type "Vector Structure" :default (1.0 1.0 1.0)) (MaxSpeed :type "Float (double-precision)" :default 500.0))
  (bind _closebadboys (`self.CloseBadBoys`))
  (set `CharacterMovementComponent.MaxWalkSpeed` MaxSpeed (`self.CharacterMovement`))
  (set `self.Direction` (0.0 0.0 0.0))
  (`KismetArrayLibrary.Array_Clear` (`self.CloseBadBoys`))
  (for _array_element (`self.OtherBadBoys`)
    (if (< (`KismetMathLibrary.Vector_Distance` (`self.K2_GetActorLocation` _array_element) (`self.K2_GetActorLocation`)) (`self.CloseDistance`))
      (`KismetArrayLibrary.Array_Add` (`self.CloseBadBoys`) _array_element)))
  (bind _direction (`self.MoveToTarget` DirectionFactor))
  (bind _direction_2 (`self.MoveCloser` _closebadboys))
  (bind _direction_3 (`self.MoveWith` _closebadboys))
  (bind _direction_4 (`self.MoveAway` _closebadboys))
  (if (!= DirectionChanger (1.0 1.0 1.0))
    (`self.AddMovementInput` DirectionChanger)
    (else
      (`self.AddMovementInput` (+ _direction_3 _direction_2 _direction _direction_4)))))

(fn `MoveAway`
  (params (CloseBadBoys :type "Array of Character Object Reference"))
  (returns (Direction :type "Vector Structure"))
  (locals (FDistance :type "Float (double-precision)") (Distance :type "Vector Structure") (Difference :type "Vector Structure") (DirectionToNeighbour :type "Vector Structure") (Away :type "Vector Structure"))
  (if (> (`KismetArrayLibrary.Array_Length` CloseBadBoys) 0)
    (set `local.Distance` (0.0 0.0 0.0))
    (for _array_element CloseBadBoys
      (bind _returnvalue (- (`self.K2_GetActorLocation`) (`self.K2_GetActorLocation` _array_element)))
      (set `local.DirectionToNeighbour` _returnvalue)
      (bind _output_get (set `local.FDistance` (`KismetMathLibrary.VSize` _returnvalue)))
      (if (and (> _output_get 0.0) (< _output_get (`self.MinDistance`)))
        (set `local.Away` (+ (`local.Away`) (* (* (`KismetMathLibrary.Normal` (`local.DirectionToNeighbour`)) (/ (`self.MinDistance`) (`local.FDistance`))) 3.0)))))
    (return (/ (`local.Away`) (`self.AwayFactor`)))
    (else
      (return (0.0 0.0 0.0)))))

(fn `MoveCloser`
  (params (CloseBadBoys :type "Array of Character Object Reference (by ref)"))
  (returns (Direction :type "Vector Structure"))
  (locals (Average :type "Vector Structure") (Closer :type "Vector Structure"))
  (bind _returnvalue (`KismetArrayLibrary.Array_Length` CloseBadBoys))
  (if (> _returnvalue 0)
    (for _array_element CloseBadBoys
      (set `local.Average` (+ (`self.K2_GetActorLocation` _array_element) (`local.Average`))))
    (return (`KismetMathLibrary.Normal` (- (/ (`local.Average`) _returnvalue) (`self.K2_GetActorLocation`))))
    (else
      (return (0.0 0.0 0.0)))))

(fn `MoveToTarget`
  (params (Factor :type "Float (double-precision)" :default 1.0))
  (returns (Direction :type "Vector Structure"))
  (bind _returnvalue (`GameplayStatics.GetActorOfClass` "/Game/Blueprints/RunBoy.RunBoy_C"))
  (bind _output_get (set `self.Direction` (+ (`self.Direction`) (/ (- (`self.K2_GetActorLocation` _returnvalue) (`self.K2_GetActorLocation`)) (`self.TargetFactor`)))))
  (return (* (`KismetMathLibrary.Normal` _output_get) Factor)))

(fn `MoveWith`
  (params (CloseBadBoys :type "Array of Character Object Reference"))
  (returns (Direction :type "Vector Structure"))
  (locals (Average :type "Vector Structure"))
  (if (> (`KismetArrayLibrary.Array_Length` CloseBadBoys) 0)
    (set `local.Average` (0.0 0.0 0.0))
    (for _array_element CloseBadBoys
      (bind _asbad_boy (cast `/Game/Blueprints/BadBoy` _array_element))
      (set `local.Average` (+ (`self.GetVelocity` _asbad_boy) (`local.Average`))))
    (return (`KismetMathLibrary.Normal` (`local.Average`)))
    (else
      (return (0.0 0.0 0.0)))))

(fn `UserConstructionScript`)