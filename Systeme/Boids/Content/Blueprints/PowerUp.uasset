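; PowerUp is a pickup actor that randomly becomes Stinky, Yummy or Confusing on BeginPlay, skipping the enum's first entry.
; The chosen state selects the material on its Cylinder.
; When a RunBoy overlaps it, it sets that character's State and hides itself.
; It destroys itself after a delay equal to the PowerupDuration read from the RunBoy_BP found in the world.
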(event `self.ReceiveBeginPlay`
  (bind _output_get (set `self.State` (select `/Game/Blueprints/RunBoy_Enum` (cast `/Game/Blueprints/RunBoy_Enum` (`KismetMathLibrary.Conv_IntToByte` (+ (`KismetMathLibrary.RandomInteger` 3) 1))) :`NewEnumerator1` "NewEnumerator1" :`NewEnumerator2` "NewEnumerator2" :`NewEnumerator3` "NewEnumerator3" :!type "/Game/Blueprints/RunBoy_Enum Enum")))
  (if (`|EnumEquality` _output_get "NewEnumerator1")
    (`PrimitiveComponent.SetMaterial` (`self.Cylinder`) 0 "/Game/Blueprints/StinkyMaterial.StinkyMaterial")
    (elif (`|EnumEquality` _output_get "NewEnumerator2")
      (`PrimitiveComponent.SetMaterial` (`self.Cylinder`) 0 "/Game/Blueprints/YummyMaterial.YummyMaterial")
      (elif (`|EnumEquality` _output_get "NewEnumerator3")
        (`PrimitiveComponent.SetMaterial` (`self.Cylinder`) 0 "/Game/Blueprints/ConfusingMaterial.ConfusingMaterial")))))

(event `self.ReceiveActorBeginOverlap`
  (params (OtherActor :type "Actor Object Reference"))
  (bind _asrun_boy (cast `/Game/Blueprints/RunBoy` OtherActor))
  (set `/Game/Blueprints/RunBoy.State` self _asrun_boy)
  (`self.SetActorHiddenInGame` true)
  (bind _returnvalue (`GameplayStatics.GetActorOfClass` "/Game/Blueprints/RunBoy_BP.RunBoy_BP_C"))
  (`KismetSystemLibrary.Delay` (`/Game/Blueprints/RunBoy_BP.PowerupDuration` _returnvalue))
  (`self.K2_DestroyActor`))

(fn `UserConstructionScript`)