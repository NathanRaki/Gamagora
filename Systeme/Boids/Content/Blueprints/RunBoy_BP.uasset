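; RunBoy_BP runs the arena spawning, keeping it stocked with BadBoy enemies and PowerUp pickups.
; From BeginPlay, a delay loop checks the BadBoy count and, below MaxBadBoys, spawns a random-sized group at one random point, so the cap can be overshot.
; GameStarted starts a looping timer for SpawnPowerup, which adds a pickup at a random arena position while fewer than five exist.
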(event `self.ReceiveBeginPlay`
  (set `self.Timer` 0.0)
  (`self.GameStarted`)
  (bind _outactors (`GameplayStatics.GetAllActorsOfClass` "/Game/Blueprints/BadBoy.BadBoy_C" :!label _label))
  (if (< (`KismetArrayLibrary.Array_Length` _outactors) (`self.MaxBadBoys`))
    (bind _output_get (set `self.XValue` (`KismetMathLibrary.RandomFloatInRange` (* (/ (`self.ArenaSize`) 2.0) -1.0) (/ (`self.ArenaSize`) 2.0))))
    (bind _output_get_2 (set `self.YValue` (`KismetMathLibrary.RandomFloatInRange` (* (/ (`self.ArenaSize`) 2.0) -1.0) (/ (`self.ArenaSize`) 2.0))))
    (for _ (range (+ (+ (`KismetMathLibrary.RandomInteger` (- (`self.MaxNumberInGroup`) 1)) 1) 1))
      (`|SpawnActorFromClass` "/Game/Blueprints/BadBoy.BadBoy_C" (`KismetMathLibrary.MakeTransform` (`KismetMathLibrary.MakeVector` _output_get _output_get_2)) "AdjustIfPossibleButAlwaysSpawn" "OverrideRootScale" null null)))
  (`KismetSystemLibrary.Delay` 0.1)
  (goto _label))

(event `GameStarted`
  (`KismetSystemLibrary.K2_SetTimer` null "SpawnPowerup" 2.0 true))

(fn `SpawnPowerup`
  (bind _outactors (`GameplayStatics.GetAllActorsOfClass` "/Game/Blueprints/PowerUp.PowerUp_C"))
  (if (< (`KismetArrayLibrary.Array_Length` _outactors) 5)
    (`|SpawnActorFromClass` "/Game/Blueprints/PowerUp.PowerUp_C" (`KismetMathLibrary.MakeTransform` (`KismetMathLibrary.MakeVector` (`KismetMathLibrary.RandomFloatInRange` (* (/ (`self.ArenaSize`) 2.0) -1.0) (/ (`self.ArenaSize`) 2.0)) (`KismetMathLibrary.RandomFloatInRange` (* (/ (`self.ArenaSize`) 2.0) -1.0) (/ (`self.ArenaSize`) 2.0)) 40.0)) "AdjustIfPossibleButAlwaysSpawn" "OverrideRootScale" null null)))

(fn `UserConstructionScript`)