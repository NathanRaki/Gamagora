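; DriveBoy draws a route line on the ground from the player's Sedan along the remaining Path points.
; Each Tick it trims Path from the point nearest the car, feeds that into a runtime spline, and rebuilds slightly raised spline meshes per segment.
; BeginPlay also parses graph.txt into NodesDict, which is unused here, and Path is never filled in this graph.
; DrawCity is a debug-print stub.
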(event `self.ReceiveBeginPlay`
  (bind _returnvalue (`AddComponent|NODE_AddSplineComponent-2`))
  (set `self.PathSplineComponent` _returnvalue)
  (bind _outactors (`GameplayStatics.GetAllActorsOfClass` "/Game/VehicleBP/Sedan/Sedan.Sedan_C"))
  (set `self.player` (`|GetArrayItem` _outactors))
  (set `self.FileRows` (`KismetStringLibrary.ParseIntoArray` (`CustomNodes.FileLoadString` (`KismetStringLibrary.Concat_StrStr` (`BlueprintPathsLibrary.GetPath` (`KismetSystemLibrary.GetProjectDirectory`)) "/graph.txt")) " \n"))
  (for _array_element (`self.FileRows`)
    (bind (_lefts _rights) (`KismetStringLibrary.Split` _array_element " "))
    (`BlueprintMapLibrary.Map_Add` (`self.NodesDict`) (`KismetStringLibrary.Conv_StringToInt` _lefts) _rights)))

(event `self.DrawCity`
  (`KismetSystemLibrary.PrintString` "Hello"))

(event `self.ReceiveTick`
  (params (DeltaSeconds :type "Float (single-precision)"))
  (bind _pathsplinecomponent (`self.PathSplineComponent`))
  (bind _draw (`self.Draw`))
  (bind _returnvalue (`SplineComponent.GetNumberOfSplinePoints` _pathsplinecomponent))
  (bind _returnvalue_2 (`self.K2_GetActorLocation` (`self.player`)))
  (if (> (`KismetArrayLibrary.Array_Length` (`self.path`)) 0)
    (`KismetArrayLibrary.Array_Clear` _draw)
    (`KismetArrayLibrary.Array_Add` _draw _returnvalue_2)
    (for (_array_element _array_index) (`self.path`)
      (bind _returnvalue_3 (`KismetMathLibrary.Vector_Distance` _array_element _returnvalue_2))
      (if (< _returnvalue_3 (`self.Min`))
        (set `self.Min` _returnvalue_3)
        (set `self.MinIndex` _array_index)))
    (set `self.Min` 1000000.0)
    (for _index (range (`self.MinIndex`) (`KismetArrayLibrary.Array_Length` (`self.path`)))
      (`KismetArrayLibrary.Array_Add` (`self.Draw`) (`|GetArrayItem` (`self.path`) _index)))
    (for _array_element_2 (`self.SplineMeshComponents`)
      (`ActorComponent.K2_DestroyComponent` _array_element_2))
    (`KismetArrayLibrary.Array_Clear` (`self.SplineMeshComponents`))
    (`SplineComponent.SetSplinePoints` _pathsplinecomponent (`self.Draw`) "World" true)
    (for _index_2 (range _returnvalue)
      (`SplineComponent.SetSplinePointType` _pathsplinecomponent _index_2 "CurveClamped" true))
    (for _index_3 (range (+ (- _returnvalue 2) 1))
      (bind _returnvalue_4 (`AddComponent|NODE_AddSplineMeshComponent-0`))
      (`KismetArrayLibrary.Array_Add` (`self.SplineMeshComponents`) _returnvalue_4)
      (bind (_location _tangent) (`SplineComponent.GetLocationAndTangentAtSplinePoint` _pathsplinecomponent _index_3 "Local"))
      (bind (_location_2 _tangent_2) (`SplineComponent.GetLocationAndTangentAtSplinePoint` _pathsplinecomponent (+ _index_3 1) "Local"))
      (`SplineMeshComponent.SetStartAndEnd` _returnvalue_4 (+ _location (0.0 0.0 5.0)) _tangent (+ _location_2 (0.0 0.0 5.0)) _tangent_2 true))))

(fn `UserConstructionScript`)