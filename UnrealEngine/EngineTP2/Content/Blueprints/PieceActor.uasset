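; Collectible coin actor that spins every tick and is picked up on overlap, with any overlapping actor speeding up its spin.
; A regular coin destroys itself after a short delay, notifies MyGameManager and plays a pickup sound.
; A self-cast detects the ChildPieceActor bonus coin, which waits longer, resets the overlapping Character's walk speed, then destroys itself without notification or sound.
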(event `self.ReceiveTick`
  (params (DeltaSeconds :type "Float (single-precision)"))
  ;[1 1 1] Rotates the coin every tick
  (if true
    (`SceneComponent.K2_AddLocalRotation` (`self.StaticMesh`) (`self.RSpin`) false false)))

(event `self.ReceiveActorBeginOverlap`
  (params (OtherActor :type "Actor Object Reference"))
  (set `self.RSpin` (struct :`Pitch` 5.0 :`Yaw` 5.0 :`Roll` 5.0)) ; Changes rotation speed
  (cast `/Game/Blueprints/ChildPieceActor` self ; Check if this is a bonus coin
    (:`then`
      ;[1 1 1] Resets the player speed after 2 seconds
      (`KismetSystemLibrary.Delay` 2.0)
      (bind _ascharacter (cast `Character` OtherActor))
      (set `CharacterMovementComponent.MaxWalkSpeed` 500.0 (`Character.CharacterMovement` _ascharacter)))
    (:`CastFailed`
      (`KismetSystemLibrary.Delay` 0.5)))
  (`self.K2_DestroyActor`)
  (cast `/Game/Blueprints/ChildPieceActor` self
    (:`CastFailed`
      (`/Game/Blueprints/GameManager.joueurRamassePiece` (`self.MyGameManager`))
      (`GameplayStatics.PlaySoundAtLocation` "/Game/Sounds/bruitpieces.bruitpieces" (`self.K2_GetActorLocation`) (struct) 1.0 1.0 0.0 null null null))))

(fn `UserConstructionScript`)