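; Game manager actor for a coin-collecting game that creates the HUD widget, starts the game paused and shows a pause screen on P.
; It counts pieces spawned and pieces collected through functions meant to be called externally, updating the score text on each pickup.
; Tick compares the two counters and shows the end-of-game screen when they match.
; A separate function attaches a flag skeletal mesh to the player's pawn.
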(event `Key|P`
  (params (Key :type "Key Structure"))
  (:`Pressed`
    (`/Game/TP3/MyWidget.AffichePause` (`self.myWidget`))))

(event `self.ReceiveBeginPlay`
  (`self.EnableInput` (`GameplayStatics.GetPlayerController` 0))
  (bind _returnvalue (`|CreateWidget` "/Game/TP3/MyWidget.MyWidget_C"))
  (bind _output_get (set `self.myWidget` _returnvalue))
  (`UserWidget.AddToViewport` _output_get 0)
  (`GameplayStatics.SetGamePaused` true))

(event `self.ReceiveTick`
  (params (DeltaSeconds :type "Float (single-precision)"))
  (if (== (`self.numPieceGagnees`) (`self.numPieceGenerees`))
    (`/Game/TP3/MyWidget.AfficheFinJeu` (`self.myWidget`))))

(fn `ajoutDrapeauJoueur`
  (`AddComponent|NODE_AddSkeletalMeshComponent-1` :`self` (`Controller.K2_GetPawn` (`GameplayStatics.GetPlayerController` 0)) :`RelativeTransform` (`KismetMathLibrary.MakeTransform` (0.0 0.0 20.0))))

(fn `ajoutPieceDansJeu`
  (`/Engine/EditorBlueprintResources/StandardMacros.IncrementFloat` (`self.numPieceGenerees`)))

(fn `joueurRamassePiece`
  (`/Engine/EditorBlueprintResources/StandardMacros.IncrementFloat` (`self.numPieceGagnees`)
    (:`  `
      (`self.MiseAJourScore`))))

(fn `MiseAJourScore`
  (`TextBlock.SetText` (`/Game/TP3/MyWidget.Score` (`self.myWidget`)) (`KismetTextLibrary.Conv_DoubleToText` (`self.numPieceGagnees`) "HalfToEven")))

(fn `UserConstructionScript`)