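; ChildPieceActor is a child pickup Blueprint that boosts a character's walk speed and credits the player with a flag on overlap.
; When a Character overlaps it, it raises that character's MaxWalkSpeed with no reset in this graph, calls AjoutDrapeauJoueur on MyGameManager, then runs the parent's overlap logic.
; Other actors exit at the cast, so the parent overlap never runs for them; BeginPlay, Tick and construction only forward to the parent.
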(event `self.ReceiveBeginPlay`
  (`parent.ReceiveBeginPlay`))

(event `self.ReceiveActorBeginOverlap`
  (params (OtherActor :type "Actor Object Reference"))
  (bind _ascharacter (cast `Character` OtherActor))
  (set `CharacterMovementComponent.MaxWalkSpeed` 1000.0 (`Character.CharacterMovement` _ascharacter))
  (`/Game/Blueprints/GameManager.ajoutDrapeauJoueur` (`self.MyGameManager`))
  (`parent.ReceiveActorBeginOverlap` OtherActor))

(event `self.ReceiveTick`
  (params (DeltaSeconds :type "Float (single-precision)"))
  (`parent.ReceiveTick` DeltaSeconds))

(fn `UserConstructionScript`
  (`parent.UserConstructionScript`))